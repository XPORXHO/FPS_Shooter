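; Zombie NPC character that chases the player, attacks in melee and dies from point damage.
; From BeginPlay it loops AI MoveTo toward player controller 0, playing an attack montage on arrival and retrying on failure, until IsDead is set.
; Pawn sensing sets walk speed when it sees a pawn.
; Damage reduces MaxHealth directly, triggering a hit reaction, or at zero a death montage that stops movement.
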(event `self.ReceiveBeginPlay`
  ;[1 1 1] Event Begin Play
  (`self.Run to player`))

(event `Run to player`
  ;[1 1 1] Following player logic
  (if (not (`self.IsDead?`))
    (`|AIMoveTo` self (0.0 0.0 0.0) (`GameplayStatics.GetPlayerController` 0) 40.0
      (:`OnSuccess`
        (`self.Attack player`))
      (:`OnFail`
        (`self.Run to player`)))))

(event `self.PawnSensing.OnSeePawn`
  (params (Pawn :type "Pawn Object Reference"))
  ;[1 1 1] Pawn sensing
  (set `CharacterMovementComponent.MaxWalkSpeed` 360.0 (`self.CharacterMovement`)))

(event `Attack player`
  ;[1 1 1] Attack Logic
  (`|PlayMontage` (`self.Mesh`) "/Game/The_Shootergame/Scary_Zombie_Pack/Animations/zombie_attack_Montage1.zombie_attack_Montage1"
    (:`OnCompleted`
      (`self.Run to player`))))

(event `self.ReceivePointDamage`
  (params (Damage :type "Float (single-precision)") (DamageType :type "DamageType Object Reference") (HitLocation :type "Vector Structure") (HitNormal :type "Vector Structure") (HitComponent :type "PrimitiveComponent Object Reference") (BoneName :type Name) (ShotFromDirection :type "Vector Structure") (InstigatedBy :type "Controller Object Reference") (DamageCauser :type "Actor Object Reference") (HitInfo :type "HitResult Structure (by ref)"))
  ;[1 1 1] Event on damage
  (if (`self.IsDead?`)
    _
    (elif (<= (`self.Max Health`) 0.0)
      (`self.death`)
      (else
        (bind _output_get (set `self.Max Health` (- (`self.Max Health`) Damage)))
        (if (<= _output_get 0.0)
          (`self.death`)
          (else
            (`|PlayMontage` (`self.Mesh`) "/Game/The_Shootergame/Scary_Zombie_Pack/Animations/Zombie_Reaction_Hit_mixamo_com_Montage.Zombie_Reaction_Hit_mixamo_com_Montage")))))))

(event `death`
  ;[1 1 1] Death Logic
  (set `self.IsDead?` true)
  (`MovementComponent.StopMovementImmediately` (`self.CharacterMovement`))
  (`|PlayMontage` (`self.Mesh`) "/Game/The_Shootergame/Scary_Zombie_Pack/Animations/zombie_dying_Montage.zombie_dying_Montage"))

(fn `UserConstructionScript`)